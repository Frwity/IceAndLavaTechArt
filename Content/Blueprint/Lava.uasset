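; Spline-based lava flow actor whose Construction Script builds a spline mesh per segment and feeds it flow and length material parameters.
; Up and down traces at segment ends detect WaterBody actors, switching segments to solid lava or a hardening blend.
; Particles are scattered along the spline, with bubbles at the last point.
; An overlap function also applies a blend material on water; the contact-smoke function is stubbed out.
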(fn `CreateLavaContactParticle`
  (params (Position :type "Vector Structure")))

(fn `LavaBeginOverlap`
  (params (OverlappedComponent :type "PrimitiveComponent Object Reference") (OtherActor :type "Actor Object Reference") (OtherComp :type "PrimitiveComponent Object Reference") (OtherBodyIndex :type Integer) (bFromSweep :type Boolean) (SweepResult :type "HitResult Structure (by ref)"))
  (cast `WaterBody` OtherActor)
  (`PrimitiveComponent.SetMaterial` OverlappedComponent 0 "/Game/Materials/Lave/M_Lava_Blend.M_Lava_Blend")
  (return))

(fn `LavaEndOverlap`
  (params (OverlappedComponent :type "PrimitiveComponent Object Reference") (OtherActor :type "Actor Object Reference") (OtherComp :type "PrimitiveComponent Object Reference") (OtherBodyIndex :type Integer)))

(fn `UserConstructionScript`
  (bind _startcumul (`self.StartCumul`))
  (bind _spline (`self.Spline`))
  (bind _currentconstructedmesh (`self.CurrentConstructedMesh`))
  (bind _splineindex (`self.SplineIndex`))
  (bind _splineindex_2 (`self.SplineIndex`))
  (bind _spline_2 (`self.Spline`))
  (bind _spline_3 (`self.Spline`))
  (bind _splineindex_3 (`self.SplineIndex`))
  (bind _spline_4 (`self.Spline`))
  (bind _spline_5 (`self.Spline`))
  (bind _spline_6 (`self.Spline`))
  (bind _currentconstructedmesh_2 (`self.CurrentConstructedMesh`))
  (bind _returnvalue (`SplineComponent.GetNumberOfSplinePoints` _spline_4))
  (bind _returnvalue_2 (`SplineComponent.GetLocationAtDistanceAlongSpline` _spline (`self.ParticleDistanceCounter`) "Local"))
  (bind _returnvalue_3 (`SplineComponent.GetLocationAtSplinePoint` _spline_2 _splineindex_3 "World"))
  (bind (_returnvalue_x _returnvalue_y) (`KismetMathLibrary.BreakVector` (* (`KismetMathLibrary.RandomUnitVector`) (`KismetMathLibrary.RandomFloatInRange` 0.0 100.0))))
  (bind _returnvalue_4 (`SplineComponent.GetLocationAtSplinePoint` _spline_2 (+ _splineindex_3 1) "World"))
  (bind _returnvalue_5 (`KismetMathLibrary.VSize` (- (`SplineComponent.GetLocationAtSplinePoint` _spline_5 _splineindex_2 "Local") (`SplineComponent.GetLocationAtSplinePoint` _spline_5 (+ _splineindex_2 1) "Local"))))
  ;[1 1 1] Loop of spline mesh component
  (`|ExecutionSequence`
    (:`then_0`
      (set `self.StartCumul` 0.0)
      (`KismetArrayLibrary.Array_Clear` (`self.Meshes`))
      (for _index (range (+ (- _returnvalue 2) 1))
        (set `self.SplineIndex` _index)
        (bind _returnvalue_6 (`AddComponent|NODE_AddSplineMeshComponent-0`))
        (set `self.CurrentConstructedMesh` _returnvalue_6)
        (set `self.FirstRay` false)
        (set `self.SecondRay` false)
        (`|ExecutionSequence`
          (:`then_0`
            ;[1 1 1] Raycast to determine where to blend into hardened lava
            (bind _outhit (`KismetSystemLibrary.LineTraceSingleByProfile` _returnvalue_3 (+ _returnvalue_3 (0.0 0.0 100.0)) "None"))
            (cast `WaterBody` (`.HitActor` (`GameplayStatics.BreakHitResult` _outhit)))
            (set `self.FirstRay` true :!label _label)
            (set `self.LavaContactPoint` (`SplineComponent.GetLocationAtSplinePoint` _spline_6 _splineindex "Local")))
          (:`then_1`
            (bind _outhit_2 (`KismetSystemLibrary.LineTraceSingleByProfile` _returnvalue_3 (+ _returnvalue_3 (0.0 0.0 -100.0)) "None"))
            (cast `WaterBody` (`.HitActor` (`GameplayStatics.BreakHitResult` _outhit_2)))
            (goto _label))
          (:`then_2`
            (bind _outhit_3 (`KismetSystemLibrary.LineTraceSingleByProfile` _returnvalue_4 (+ _returnvalue_4 (0.0 0.0 -100.0)) "None"))
            (cast `WaterBody` (`.HitActor` (`GameplayStatics.BreakHitResult` _outhit_3)))
            (set `self.SecondRay` true :!label _label_2)
            (set `self.LavaContactPoint` (`SplineComponent.GetLocationAtSplinePoint` _spline_6 (+ _splineindex 1) "Local")))
          (:`then_3`
            (bind _outhit_4 (`KismetSystemLibrary.LineTraceSingleByProfile` _returnvalue_4 (+ _returnvalue_4 (0.0 0.0 100.0)) "None"))
            (cast `WaterBody` (`.HitActor` (`GameplayStatics.BreakHitResult` _outhit_4)))
            (goto _label_2))
          (:`then_4`
            ;[1 1 1] Material set and parameters
            (if (and (`self.FirstRay`) (`self.SecondRay`))
              (`PrimitiveComponent.SetMaterial` _currentconstructedmesh_2 0 "/Game/Materials/Lave/MI_Lava_Solid.MI_Lava_Solid")
              (elif (`self.FirstRay`)
                (`PrimitiveComponent.SetMaterial` _currentconstructedmesh_2 0 "/Game/Materials/Lave/MI_Lava_Blend.MI_Lava_Blend" :!label _label_3)
                (`self.CreateLavaContactParticle` (`self.LavaContactPoint`))
                (elif (`self.SecondRay`)
                  (goto _label_3)
                  (else
                    _))))
            (`|ExecutionSequence`
              (:`then_0`
                (`MeshComponent.SetScalarParameterValueOnMaterials` _currentconstructedmesh "Length" _returnvalue_5))
              (:`then_1`
                (`MeshComponent.SetScalarParameterValueOnMaterials` _currentconstructedmesh "Start" _startcumul))
              (:`then_2`
                (`MeshComponent.SetScalarParameterValueOnMaterials` _currentconstructedmesh "Speed" (`self.FlowSpeed`)))
              (:`then_3`
                (`MeshComponent.SetScalarParameterValueOnMaterials` _currentconstructedmesh "HardenedBlend" (`self.HardenedBlend`)))
              (:`then_4`
                (set `self.StartCumul` (+ _returnvalue_5 _startcumul)))))
          (:`then_5`
            (bind _returnvalue_7 (+ _index 1))
            ;[1 1 1] Set Spline mesh component pos
            (`SplineMeshComponent.SetStartAndEnd` (`self.CurrentConstructedMesh`) (`SplineComponent.GetLocationAtSplinePoint` _spline_3 _index "Local") (`SplineComponent.GetTangentAtSplinePoint` _spline_3 _index "Local") (`SplineComponent.GetLocationAtSplinePoint` _spline_3 _returnvalue_7 "Local") (`SplineComponent.GetTangentAtSplinePoint` _spline_3 _returnvalue_7 "Local") true))))
      (`AddComponent|NODE_AddParticleSystemComponent-9` :`RelativeTransform` (`KismetMathLibrary.Conv_VectorToTransform` (`SplineComponent.GetLocationAtSplinePoint` _spline_4 (- _returnvalue 1) "Local")) :!pinned true) ; Bubble
    )
    (:`then_1`
      ;[1 1 1] Particle
      (set `self.ParticleDistanceCounter` 0.0)
      (while (< (`self.ParticleDistanceCounter`) (`SplineComponent.GetSplineLength` _spline))
        (`AddComponent|NODE_AddParticleSystemComponent-6` :`RelativeTransform` (`KismetMathLibrary.Conv_VectorToTransform` _returnvalue_2))
        (`AddComponent|NODE_AddParticleSystemComponent-8` :`RelativeTransform` (`KismetMathLibrary.Conv_VectorToTransform` (+ _returnvalue_2 (`KismetMathLibrary.MakeVector` _returnvalue_x _returnvalue_y))))
        (set `self.ParticleDistanceCounter` (+ (`self.ParticleDistanceCounter`) (`self.DistanceBetweenParticle`)))))))