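; Boat actor that follows a BoatTrack spline, disturbs the fluid sim and breaks ice along its path.
; A timeline drives XY and yaw along the spline, preserving Z, pitch and roll, with Buoyancy ticking.
; An oscillating ForceMesh is registered as a dynamic force with BP_FluidSim_01.
; BreakIce periodically adds two scaled static meshes above and ahead of the hull, apparently runtime virtual texture stamps, without removing them.
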(event `self.ReceiveBeginPlay`
  (`KismetSystemLibrary.Delay` 0.1)
  (bind _returnvalue (`GameplayStatics.GetActorOfClass` "/Water/FluidSimulation/Blueprints/BP_FluidSim_01.BP_FluidSim_01_C"))
  (set `self.Sim` _returnvalue)
  (`/Water/FluidSimulation/Blueprints/BP_FluidSim_01.Register Dynamic Force` (`self.Sim`) (make `/Water/FluidSimulation/Blueprints/Structs/FluidForceDynamic` "NewEnumerator0" (`self.Radius`) (`self.Strength`) (`self.ForceMesh`) (`self.Material`) (make `/Water/FluidSimulation/Blueprints/Structs/FluidForceSocketInfo` (`|MakeMap` "None" :!type "Name" :!valuetype "Name"))) (`self.ForceMesh`) 0.0))

(event `self.ReceiveTick`
  (params (DeltaSeconds :type "Float (single-precision)"))
  (`ActorComponent.SetComponentTickEnabled` (`self.Buoyancy`) true)
  (`self.BreakIce`)
  (`SceneComponent.K2_SetRelativeLocation` (`self.ForceMesh`) (+ (`KismetMathLibrary.MakeVector` (* (`KismetMathLibrary.Sin` (* (`KismetSystemLibrary.GetGameTimeInSeconds`) (`self.Oscillation Speed`))) (`self.Osc Mag`))) (`self.Offset`)) false false)
  (`TimelineComponent.SetPlayRate` (`self.BoatMover`) (/ 1.0 (`self.Duration`)))
  (bind (_direction _alpha) (`Timeline|BoatMover`)
    (:`Update`
      (set `self.Alpha` _alpha)
      (`self.MoveBoat`))))

(fn `BreakIce`
  (bind _boatmesh (`self.boatMesh`))
  (bind _returnvalue (+ (`SceneComponent.K2_GetComponentLocation` _boatmesh) (0.0 0.0 650.0)))
  (if (> (`self.rvttimer`) 0.025)
    (bind _returnvalue_2 (`AddComponent|NODE_AddStaticMeshComponent-1` :`bManualAttachment` true :`RelativeTransform` (`KismetMathLibrary.Conv_VectorToTransform` _returnvalue)))
    (`SceneComponent.SetWorldScale3D` _returnvalue_2 (8.0 8.0 8.0))
    (`SceneComponent.K2_SetWorldRotation` _returnvalue_2 (`SceneComponent.K2_GetComponentRotation` (`self.boatMesh`)) false false)
    (bind _returnvalue_3 (`AddComponent|NODE_AddStaticMeshComponent-0` :`bManualAttachment` true :`RelativeTransform` (`KismetMathLibrary.Conv_VectorToTransform` (+ _returnvalue (* (`SceneComponent.GetForwardVector` _boatmesh) 700.0)))))
    (`SceneComponent.SetWorldScale3D` _returnvalue_3 (3.0 3.0 3.0))
    (`SceneComponent.K2_SetWorldRotation` _returnvalue_3 (`SceneComponent.K2_GetComponentRotation` (`self.boatMesh`)) false false)
    (set `self.rvttimer` 0.0)
    (else
      (set `self.rvttimer` (+ (`self.rvttimer`) (`GameplayStatics.GetWorldDeltaSeconds`))))))

(fn `MoveBoat`
  (bind (_returnvalue_x _returnvalue_y _returnvalue_z) (`KismetMathLibrary.BreakVector` (`self.K2_GetActorLocation`)))
  (bind (_returnvalue_roll _returnvalue_pitch) (`KismetMathLibrary.BreakRotator` (`self.K2_GetActorRotation`)))
  (bind _track (`/Game/Blueprint/BoatTrack.Track` (`self.BoatTrack`)))
  (bind _returnvalue (`KismetMathLibrary.Lerp` 0.0 (`SplineComponent.GetSplineLength` _track) (`self.Alpha`)))
  (bind (_returnvalue_x_2 _returnvalue_y_2) (`KismetMathLibrary.BreakVector` (`SplineComponent.GetLocationAtDistanceAlongSpline` _track _returnvalue "World")))
  (bind (_returnvalue_roll_2 _returnvalue_pitch_2 _returnvalue_yaw) (`KismetMathLibrary.BreakRotator` (`SplineComponent.GetRotationAtDistanceAlongSpline` _track _returnvalue "World")))
  (`self.K2_SetActorLocationAndRotation` (`KismetMathLibrary.MakeVector` _returnvalue_x_2 _returnvalue_y_2 _returnvalue_z) (`KismetMathLibrary.MakeRotator` _returnvalue_roll _returnvalue_pitch _returnvalue_yaw)))

(fn `UserConstructionScript`
  (set `self.Offset` (`SceneComponent.RelativeLocation` (`self.ForceMesh`)))
  (`SceneComponent.SetRelativeScale3D` (`self.ForceMesh`) (`KismetMathLibrary.Conv_DoubleToVector` (* (`self.Radius`) 1.0)))
  (`SceneComponent.SetHiddenInGame` (`self.ForceMesh`) (not (`self.ShowForceMesh`)) false))